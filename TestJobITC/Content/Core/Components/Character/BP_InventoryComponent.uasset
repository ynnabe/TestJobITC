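; BP_InventoryComponent is a character component that holds a fixed-slot inventory of item data.
; On BeginPlay it resizes the Inventory array to InventorySize, leaving empty slots as invalid entries.
; TryToAddItem places an item in the first empty slot and returns whether it succeeded.
; Every Tick, PrintInventory prints each slot's index and item name, or Not valid, on screen as a debug readout.
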(event `self.ReceiveBeginPlay`
  (`KismetArrayLibrary.Array_Resize` (`self.Inventory`) (`self.InventorySize`)))

(event `self.ReceiveTick`
  (params (DeltaSeconds :type "Float (single-precision)"))
  (`self.PrintInventory`))

(fn `PrintInventory`
  (bind _returnvalue (`GameplayStatics.GetWorldDeltaSeconds`))
  (for (_array_element _array_index) (`self.Inventory`)
    (`/Engine/EditorBlueprintResources/StandardMacros.IsValid` _array_element
      (:`Is Valid`
        (`KismetSystemLibrary.PrintString` (`KismetStringLibrary.Concat_StrStr` (`KismetStringLibrary.Conv_IntToString` _array_index) " " (`KismetStringLibrary.Conv_NameToString` (`/Game/Core/Items/BP_DataItem.Name` _array_element))) true true (struct :`G` 0.66 :`B` 1.0 :`A` 1.0) _returnvalue))
      (:`Is Not Valid`
        (`KismetSystemLibrary.PrintString` (`KismetStringLibrary.Concat_StrStr` (`KismetStringLibrary.Conv_IntToString` _array_index) " Not valid") true true (struct :`G` 0.66 :`B` 1.0 :`A` 1.0) _returnvalue)))))

(fn `TryToAddItem`
  (params (ItemData :type "/Game/Core/Items/BP_DataItem Object Reference"))
  (returns (Success :type Boolean))
  (for (_array_element _array_index) (`self.Inventory`)
    (if (not (`KismetSystemLibrary.IsValid` _array_element))
      (`KismetArrayLibrary.Array_Set` (`self.Inventory`) _array_index (`local.ItemData`))
      (return true)))
  (return false))