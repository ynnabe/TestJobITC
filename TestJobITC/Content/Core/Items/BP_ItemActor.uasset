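; BP_ItemActor is a world item actor that a player can pick up into their inventory.
; Its construction script creates an ItemData object from ItemDataClass, passing in Name, and applies Mesh to the static mesh component.
; On Interact, it passes ItemData to the player's BPInventoryComponent, destroying itself if the add succeeds and printing a debug message for either result.
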(event `/Game/Core/Interface/BI_Interactable.Interact`
  (params (Player :type "/Game/Core/Character/BP_FirstPersonCharacter Object Reference"))
  (bind _success (`/Game/Core/Components/Character/BP_InventoryComponent.TryToAddItem` (`/Game/Core/Character/BP_FirstPersonCharacter.BP_InventoryComponent` Player) (`self.ItemData`)))
  (if _success
    (`self.K2_DestroyActor`)
    (`KismetSystemLibrary.PrintString` "Item added" true true (struct :`R` 0.000554 :`G` 1.0 :`A` 1.0))
    (else
      (`KismetSystemLibrary.PrintString` "Item not added" true true (struct :`R` 1.0 :`G` 0.015653 :`A` 1.0)))))

(fn `UserConstructionScript`
  (bind _returnvalue (`|GenericCreateObject` (`self.ItemDataClass`) (`self.Name`)))
  (set `self.ItemData` _returnvalue)
  (`StaticMeshComponent.SetStaticMesh` (`self.StaticMesh`) (`self.Mesh`)))